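; BP_Zombie2 is an enemy that chases the first-person player and damages them on contact.
; Tick re-issues an AI MoveTo toward the player's current location every frame.
; Overlapping the player subtracts a fixed amount from their CurrantHealth, while a capsule hit with the player destroys the zombie.
; Score and lose-screen logic is present but disconnected, so it never runs.
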(event `self.ReceiveActorBeginOverlap`
  (params (OtherActor :type "Actor Object Reference"))
  (`|ExecutionSequence`
    (:`then_0`
      (bind _asbp_first_person_character (cast `/Game/FirstPerson/Blueprints/BP_FirstPersonCharacter` (`GameplayStatics.GetPlayerCharacter` 0))))
    (:`then_1`
      (bind _asbp_first_person_character_2 (cast `/Game/FirstPerson/Blueprints/BP_FirstPersonCharacter` OtherActor))
      (set `/Game/FirstPerson/Blueprints/BP_FirstPersonCharacter.Currant Health` (- (`/Game/FirstPerson/Blueprints/BP_FirstPersonCharacter.Currant Health` _asbp_first_person_character_2) 20.0) _asbp_first_person_character_2))))

(event `self.ReceiveTick`
  (params (DeltaSeconds :type "Float (single-precision)"))
  (`|AIMoveTo` self (`self.K2_GetActorLocation` (`GameplayStatics.GetPlayerCharacter` 0)) null))

(event `self.Capsule.OnComponentHit`
  (params (HitComponent :type "PrimitiveComponent Object Reference") (OtherActor :type "Actor Object Reference") (OtherComp :type "PrimitiveComponent Object Reference") (NormalImpulse :type "Vector Structure") (Hit :type "HitResult Structure (by ref)"))
  (cast `/Game/FirstPerson/Blueprints/BP_FirstPersonCharacter` OtherActor)
  (`self.K2_DestroyActor`))

(fn `UserConstructionScript`)