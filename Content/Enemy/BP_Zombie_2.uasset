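; BP_Zombie_2 is an enemy zombie that chases the player and hurts them on contact.
; Every tick it issues an AI move toward the player character's location.
; Overlapping the player subtracts a fixed amount of health, and at zero it shows the lose screen and pauses the game.
; A first-person projectile hitting its ZombieAttack component destroys the zombie in one hit.
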(event `self.ReceiveActorBeginOverlap`
  (params (OtherActor :type "Actor Object Reference"))
  (bind _asbp_first_person_character (cast `/Game/FirstPerson/Blueprints/BP_FirstPersonCharacter` OtherActor))
  (bind _currant_health (`/Game/FirstPerson/Blueprints/BP_FirstPersonCharacter.Currant Health` _asbp_first_person_character))
  (set `/Game/FirstPerson/Blueprints/BP_FirstPersonCharacter.Currant Health` (- _currant_health 20.0) _asbp_first_person_character)
  (if (<= _currant_health 0.0)
    (bind _returnvalue (`|CreateWidget` "/Game/UI/Win_and_Lose_Conditions/Lose/WB_Lose_Screen.WB_Lose_Screen_C"))
    (`UserWidget.AddToViewport` _returnvalue 0)
    (`GameplayStatics.SetGamePaused` true)))

(event `self.ReceiveTick`
  (params (DeltaSeconds :type "Float (single-precision)"))
  (`|AIMoveTo` self (`self.K2_GetActorLocation` (`GameplayStatics.GetPlayerCharacter` 0)) null))

(event `self.Zombie Attack.OnComponentHit`
  (params (HitComponent :type "PrimitiveComponent Object Reference") (OtherActor :type "Actor Object Reference") (OtherComp :type "PrimitiveComponent Object Reference") (NormalImpulse :type "Vector Structure") (Hit :type "HitResult Structure (by ref)"))
  (cast `/Game/FirstPerson/Blueprints/BP_FirstPersonProjectile` OtherActor)
  (`self.K2_DestroyActor`))

(fn `UserConstructionScript`)